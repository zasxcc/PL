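; BP_EnemyCharacter is an enemy character Blueprint that takes the player as its target and shows on-screen debug readouts.
; On BeginPlay it casts player 0's character to PLCharacter and sets it as the current target.
; Every Tick it prints the angle to the target, the last damage received and HP from the PL statistic component.
; The construction script and overlap event are empty.
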(event EventBeginPlay
  (bind _asplcharacter (Utilities|Casting|CastToPLCharacter (Game|GetPlayerCharacter 0)))
  (Class|PLCharacter|SetCurrentTargetCharacter _asplcharacter))

(event Collision|EventActorBeginOverlap
  (params (OtherActor :type Actor%20Object%20Reference)))

(event EventTick
  (params (DeltaSeconds :type Float%20%28single-precision%29))
  (Development|PrintString (Utilities|String|ToString(Float) (Class|PLCharacter|GetAngletoTarget)) true true "(R=1.000000,G=0.000000,B=0.104317,A=1.000000)" 0.0)
  (Development|PrintString (Utilities|String|ToString(Float) (.damage (Class|PLCharacter|GetLastDamageInfo))) true true "(R=1.000000,G=0.447351,B=0.437404,A=1.000000)" 0.0)
  (Development|PrintString (Utilities|String|ToString(Float) (.value (.Value (Utilities|Map|Find (Variables|/Script/ProjectLight.PLStatisticComponent|GetCharacterStat (Class|PLCharacter|GetPLStatisticComponent)) "(TagName=\"Stat.HP\")")))) true true "(R=0.112205,G=1.000000,B=0.000000,A=1.000000)" 0.0))

(fn ConstructionScript)