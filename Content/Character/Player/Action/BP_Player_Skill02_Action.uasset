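; BP_Player_Skill02_Action is the action Blueprint for the player's second skill, gating its execution on a stat cost.
; CanExecuteAction calls the parent check without using its result, then compares the owner's current NeedStat value in the PLStatisticComponent against NeedResource.
; When the stat suffices, the check itself deducts the cost with regen delay applied and returns true; otherwise it returns false.
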(fn CanExecuteAction
  (params (owner :type PL%20Character%20Object%20Reference))
  (bind _returnvalue (Class|PLCharacter|GetPLStatisticComponent owner))
  (|CallParentFunction owner)
  (if (>= (.value (Class|PLStatisticComponent|GetCurrentCharacterStat _returnvalue (Variables|PLAction|GetNeedStat))) (Variables|PLAction|GetNeedResource))
    (Class|PLStatisticComponent|ModifyStat _returnvalue (Variables|PLAction|GetNeedStat) (* (Variables|PLAction|GetNeedResource) -1.0) true)
    (return true)
    (else
      (return false))))