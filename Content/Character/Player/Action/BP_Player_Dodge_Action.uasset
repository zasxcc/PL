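; Player dodge action that makes the owner immortal and disables further dodging on its player controller while active, restoring both when it ends.
; GetMontageSectionName picks the directional montage section by polling raw WASD key states rather than movement input.
; Its nested branches resolve diagonals by priority: S+D gives Right, otherwise S gives Back, D Right, A Left, and anything else Front.
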(event EventOnActionStarted
  (|CallParentFunction)
  (bind _ownercharacter (Variables|Default|GetOwnerCharacter)
    (:then
      (Class|PLCharacter|SetIsImmortality _ownercharacter true)
      (bind _asplplayer_character (Utilities|Casting|CastToPLPlayerCharacter _ownercharacter))
      (Class|PLPlayerController|SetEnableDodge (Class|PLPlayerCharacter|GetPLPlayerController _asplplayer_character) false))
    (:else)))

(event EventOnActionEnded
  (|CallParentFunction)
  (bind _ownercharacter (Variables|Default|GetOwnerCharacter)
    (:then
      (Class|PLCharacter|SetIsImmortality _ownercharacter false)
      (bind _asplplayer_character (Utilities|Casting|CastToPLPlayerCharacter _ownercharacter))
      (Class|PLPlayerController|SetEnableDodge (Class|PLPlayerCharacter|GetPLPlayerController _asplplayer_character) true))
    (:else)))

(fn GetMontageSectionName
  (bind _ownercharacter (Variables|Default|GetOwnerCharacter))
  (bind _returnvalue (Pawn|GetLocalViewingPlayerController _ownercharacter))
  (bind _returnvalue_2 (Game|Player|IsInputKeyDown _returnvalue "W"))
  (bind _returnvalue_3 (Game|Player|IsInputKeyDown _returnvalue "S"))
  (bind _returnvalue_4 (Game|Player|IsInputKeyDown _returnvalue "D"))
  (bind _returnvalue_5 (Game|Player|IsInputKeyDown _returnvalue "A"))
  (if (and _returnvalue_3 _returnvalue_4)
    (return "Right")
    (elif _returnvalue_3
      (return "Back")
      (elif _returnvalue_4
        (return "Right")
        (else
          (if (and _returnvalue_3 _returnvalue_5)
            _
            (elif _returnvalue_5
              _
              (elif _returnvalue_3
                (return "Back")
                (else
                  (if (and _returnvalue_4 _returnvalue_2)
                    _
                    (elif _returnvalue_4
                      _
                      (elif _returnvalue_2
                        (return "Front")
                        (elif (and _returnvalue_5 _returnvalue_2)
                          (return "Left")
                          (else
                            (if _returnvalue_5
                              _
                              (elif _returnvalue_2
                                _
                                (else
                                  (return "Front"))))
                            (return "Front"))))))
                  (return "Right")))))
          (return "Left"))))))