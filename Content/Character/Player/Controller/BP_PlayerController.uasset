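; Player controller that turns axis and mouse input into movement, camera look and a melee-style attack for the player character.
; Move axes feed movement input relative to control rotation, with forward flattened to yaw, while turn axes are scaled by frame delta time.
; Left click plays the first combo attack action only when no action is current.
; GetDesiredVelocity builds a normalized yaw-relative direction, using the forward axis for both components.
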(event EventBeginPlay)

(event EventTick
  (params (DeltaSeconds :type Float%20%28single-precision%29)))

(event Input|AxisEvents|InputAxisTurnPitch
  (params (AxisValue :type Float%20%28single-precision%29))
  (Class|PlayerController|AddPitchInput (* AxisValue 3e+01 (Utilities|Time|GetWorldDeltaSeconds))))

(event Input|AxisEvents|InputAxisTurnYaw
  (params (AxisValue :type Float%20%28single-precision%29))
  (Class|PlayerController|AddYawInput (* AxisValue 3e+01 (Utilities|Time|GetWorldDeltaSeconds))))

(event Input|AxisEvents|InputAxisMoveForward
  (params (AxisValue :type Float%20%28single-precision%29))
  (bind _returnvalue (Game|GetPlayerCharacter 0))
  (Utilities|IsValid _returnvalue
    (:Is%20Valid
      (Pawn|Input|AddMovementInput _returnvalue (Math|Vector|GetForwardVector (Math|Rotator|MakeRotator 0.0 0.0 (.Yaw (Math|Rotator|BreakRotator (Pawn|GetControlRotation :!class /Script/Engine.Controller))))) AxisValue false))))

(event Input|AxisEvents|InputAxisMoveRight
  (params (AxisValue :type Float%20%28single-precision%29))
  (bind _returnvalue (Game|GetPlayerCharacter 0))
  (Utilities|IsValid _returnvalue
    (:Is%20Valid
      (Pawn|Input|AddMovementInput _returnvalue (Math|Vector|GetRightVector (Pawn|GetControlRotation :!class /Script/Engine.Controller)) AxisValue false))))

(event Input|MouseEvents|LeftMouseButton
  (params (Key :type Key%20Structure :default "None"))
  (:Pressed
    (bind _asplplayer_character (Utilities|Casting|CastToPLPlayerCharacter (Game|GetPlayerCharacter 0)))
    (Utilities|IsValid (Variables|/Script/ProjectLight.PLActionManagerComponent|GetCurrentAction (Class|PLCharacter|GetPLActionComponent _asplplayer_character))
      (:Is%20Not%20Valid
        (Class|PLCharacter|PlayAction _asplplayer_character "(TagName=\"Action.Player.Attack.Combo01\")")))))

(fn ConstructionScript)

(fn GetDesiredVelocity
  (bind _returnvalue (Pawn|GetControlRotation :!class /Script/Engine.Controller))
  (bind _returnvalue_2 (Input|AxisValues|GetMoveForward))
  (return (Math|Vector|Normalize (+ (* _returnvalue_2 (Math|Vector|GetForwardVector (Math|Rotator|MakeRotator 0.0 0.0 (.yaw _returnvalue)))) (* (Math|Vector|GetRightVector (Math|Rotator|MakeRotator 0.0 0.0 (.yaw _returnvalue))) _returnvalue_2)))))