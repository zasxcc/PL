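; BP_Dragon is a dragon enemy character Blueprint that manages a collision sphere positioned relative to its head.
; The construction script places the Sphere at the head socket's X and Y, at a fixed offset below the actor's origin.
; Each tick, after the parent logic, it disables the Sphere's collision while an animation montage plays and restores query-only collision otherwise.
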(event EventBeginPlay
  (|CallParentFunction) ; 지금 이 노드는 비활성 상태입니다. \n핀을 끌어서 다른 노드를 연결하면 활성화됩니다.
)

(event Collision|EventActorBeginOverlap
  (params (OtherActor :type Actor%20Object%20Reference))
  (|CallParentFunction OtherActor) ; 지금 이 노드는 비활성 상태입니다. \n핀을 끌어서 다른 노드를 연결하면 활성화됩니다.
)

(event EventTick
  (params (DeltaSeconds :type Float%20%28single-precision%29))
  (bind _sphere (Variables|Default|GetSphere))
  (|CallParentFunction DeltaSeconds)
  (if (Animation|Montage|MontageIsPlaying (Class|PLCharacter|GetPLAnimationInstance) 0)
    (Collision|SetCollisionEnabled _sphere "NoCollision")
    (else
      (Collision|SetCollisionEnabled _sphere "QueryOnly"))))

(fn ConstructionScript
  (bind _mesh (Variables|Character|GetMesh))
  (bind _returnvalue (Transformation|GetSocketLocation _mesh "Dragon11_Head1"))
  (|CallParentFunction)
  (Transformation|SetWorldLocation (Variables|Default|GetSphere) (Math|Vector|MakeVector (.x _returnvalue) (.y _returnvalue) (- (.z (Transformation|GetActorLocation)) 1.5e+02)) false false))