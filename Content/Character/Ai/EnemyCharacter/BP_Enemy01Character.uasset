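; BP_Enemy01Character is an enemy AI character that keeps its stats across spawn and despawn by its OptimizeSubjectComponent.
; On pre-despawn it writes the statistic component's CharacterStat into the AOStat of a BP_OptimizeData object.
; On post-spawn it restores CharacterStat from that data.
; Damage handling only forwards to the parent, and BeginPlay, Tick and overlap events are empty.
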(event OnPreDespawn(OptimizeSubjectComponent)
  (params (Data :type Optimize%20Data%20Object%20Reference))
  ;[1 1 1] 디스폰시의 이벤트
  (bind _asbp_optimize_data (Utilities|Casting|CastToBP_OptimizeData Data))
  (Variables|/Game/Character/Ai/BP_OptimizeData.BP_OptimizeData_C|SetAO_Stat _asbp_optimize_data (Variables|/Script/ProjectLight.PLStatisticComponent|GetCharacterStat (Class|PLCharacter|GetPLStatisticComponent))))

(event OnPostSpawned(OptimizeSubjectComponent)
  (params (Data :type Optimize%20Data%20Object%20Reference))
  ;[1 1 1] 스폰시의 이벤트
  (bind _asbp_optimize_data (Utilities|Casting|CastToBP_OptimizeData Data))
  (Variables|/Script/ProjectLight.PLStatisticComponent|SetCharacterStat (Class|PLCharacter|GetPLStatisticComponent) (Variables|/Game/Character/Ai/BP_OptimizeData.BP_OptimizeData_C|GetAO_Stat _asbp_optimize_data)))

(event EventBeginPlay)

(event Collision|EventActorBeginOverlap
  (params (OtherActor :type Actor%20Object%20Reference)))

(event EventTick
  (params (DeltaSeconds :type Float%20%28single-precision%29)))

(event EventDamageReceiveEvent
  (params (_dealer :type PL%20Character%20Object%20Reference))
  (|CallParentFunction _dealer))

(fn ConstructionScript)