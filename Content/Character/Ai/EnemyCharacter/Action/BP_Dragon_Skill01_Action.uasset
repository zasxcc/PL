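; Action Blueprint for the dragon enemy's Skill01 that drives a flickering light effect on the owning boss.
; On action start it casts the owner to PLBossCharacter and begins a timed fast flicker of its light.
; On action end it stops the flickering point light; tick only calls the parent.
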(event EventOnActionStarted
  (|CallParentFunction)
  (bind _asplboss_character (Utilities|Casting|CastToPLBossCharacter (Variables|Default|GetOwnerCharacter)))
  (Class|PLBossCharacter|SetFlickeringLightFlicker _asplboss_character 5.0 0.1))

(event EventOnTick
  (params (DeltaTime :type Float%20%28single-precision%29))
  (|CallParentFunction DeltaTime))

(event EventOnActionEnded
  (|CallParentFunction)
  (bind _asplboss_character (Utilities|Casting|CastToPLBossCharacter (Variables|Default|GetOwnerCharacter)))
  (Class|PLBossCharacter|StopFlickeringPointLight _asplboss_character true))